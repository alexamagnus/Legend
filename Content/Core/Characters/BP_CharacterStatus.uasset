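; BP_CharacterStatus holds a character's current and maximum HP and EXP values.
; A setter function stores all four values at once without clamping or validation.
; A getter function returns HP and EXP as ratios by normalizing each current value between zero and its maximum.
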(fn GetRangeHPandExp
  (return (Math|Float|NormalizetoRange (Variables|Default|GetCurrent%20HP) 0.0 (Variables|Default|GetMax%20HP)) (Math|Float|NormalizetoRange (Variables|Default|GetCurrent%20EXP) 0.0 (Variables|Default|GetMax%20EXP))))

(fn SetHPandExp
  (params (Current%20HP :type Float%20%28double-precision%29) (Max%20HP :type Float%20%28double-precision%29) (Current%20EXP :type Float%20%28double-precision%29) (Max%20EXP :type Float%20%28double-precision%29))
  (Variables|Default|SetCurrent%20HP Current%20HP)
  (Variables|Default|SetMax%20HP Max%20HP)
  (Variables|Default|SetCurrent%20EXP Current%20EXP)
  (Variables|Default|SetMax%20EXP Max%20EXP))