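; Snail enemy that slowly patrols back and forth along the X axis and hurts the player on contact.
; Each Tick, Move steps a counter toward a signed limit while adding movement input, so patrol length is counted in frames.
; At the limit it negates the limit, resets the counter and rotates the sprite to turn around.
; Box overlap with BP_PlayerCharacter applies damage, launches the player and plays a sound.
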(event OnComponentBeginOverlap(Box)
  (params (OverlappedComponent :type Primitive%20Component%20Object%20Reference) (OtherActor :type Actor%20Object%20Reference) (OtherComp :type Primitive%20Component%20Object%20Reference) (OtherBodyIndex :type Integer) (bFromSweep :type Boolean) (SweepResult :type Hit%20Result%20Structure%20%28by%20ref%29))
  (bind _asbp_player_character (Utilities|Casting|CastToBP_PlayerCharacter OtherActor))
  (Game|Damage|ApplyDamage _asbp_player_character 1.0 0 0)
  (Character|LaunchCharacter _asbp_player_character (Variables|Default|GetLaunch%20Velocity) true false)
  (Audio|PlaySound2D "/Game/Sounds/Enemy/Snail/SW_Snail.SW_Snail" 1.0 1.0 0.0 0 0))

(event Custom|Move
  (bind _sprite (Variables|Default|GetSprite))
  (Math|Float|CompareFloat (Variables|Default|Gets1) (Variables|Default|Gets)
    (:>
      (Pawn|Input|AddMovementInput "-1.000000,0.000000,0.000000" 0.1 false)
      (bind _result (Math|Float|DecrementFloat (Variables|Default|Gets1))
        (:%20%20
          (Variables|Default|Sets1 _result))))
    (:==
      (if (> (Variables|Default|Gets) 0.0)
        (Variables|Default|Sets (* (Variables|Default|Gets) -1.0))
        (Variables|Default|Sets1 0.0)
        (Transformation|SetRelativeRotation _sprite "0, 0, 0" false false)
        (else
          (Variables|Default|Sets (* (Variables|Default|Gets) -1.0))
          (Variables|Default|Sets1 0.0)
          (Transformation|SetRelativeRotation _sprite "0.000000,180.000000,0.000000" false false))))
    (:<
      (Pawn|Input|AddMovementInput "1.000000,0.000000,0.000000" 0.1 false)
      (bind _result_2 (Math|Float|IncrementFloat (Variables|Default|Gets1))
        (:%20%20
          (Variables|Default|Sets1 _result_2))))))

(event EventTick
  (params (DeltaSeconds :type Float%20%28single-precision%29))
  (CallFunction|Move))

(fn ConstructionScript)