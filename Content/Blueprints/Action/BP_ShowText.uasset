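; BP_ShowText is a trigger volume actor that shows a text message on screen while something overlaps its box.
; Begin overlap creates a WBP_ShowText widget from the Text variable and adds it to the viewport; end overlap removes it and clears the reference.
; Neither event filters the overlapping actor.
; The construction script sizes the box from the InBoxExtent variable, so each placed instance can have its own extent.
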(event OnComponentBeginOverlap(Box)
  (params (OverlappedComponent :type Primitive%20Component%20Object%20Reference) (OtherActor :type Actor%20Object%20Reference) (OtherComp :type Primitive%20Component%20Object%20Reference) (OtherBodyIndex :type Integer) (bFromSweep :type Boolean) (SweepResult :type Hit%20Result%20Structure%20%28by%20ref%29))
  (bind _returnvalue (UserInterface|CreateWidget "/Game/UI/WBP_ShowText.WBP_ShowText_C" 0 (Variables|Setupss|GetText)))
  (bind _output_get (Variables|Inst|SetShow%20text _returnvalue))
  (UserInterface|Viewport|AddtoViewport _returnvalue 0))

(event OnComponentEndOverlap(Box)
  (params (OverlappedComponent :type Primitive%20Component%20Object%20Reference) (OtherActor :type Actor%20Object%20Reference) (OtherComp :type Primitive%20Component%20Object%20Reference) (OtherBodyIndex :type Integer))
  (Widget|RemovefromParent (Variables|Inst|GetShow%20text))
  (Variables|Inst|SetShow%20text 0))

(fn ConstructionScript
  (Components|Box|SetBoxExtent (Variables|Default|GetBox) (Variables|Setupss|GetIn%20Box%20Extent) true))